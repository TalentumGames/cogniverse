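; Player controller for the Penguins board game, linking a player's HUD and piece placement to the shared game state.
; On BeginPlay, the local controller creates the WB_Penguins HUD and sets Game-and-UI input.
; Server_PlacePiece passes the PlayerState's side and a row and column to GameState's PlaceAt, printing the result.
; UpdateSide pushes the side to the HUD, and PreLoadSide does so from PlayerState if one is already assigned.
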(event `self.ReceiveBeginPlay`
  (if (`self.IsLocalPlayerController`)
    (`|ExecutionSequence`
      (:`then_0`
        (bind _returnvalue (`|CreateWidget` "/Game/Widgets/Penguins/WB_Penguins.WB_Penguins_C" self))
        (bind _output_get (set `self.HUD` _returnvalue))
        (`UserWidget.AddToViewport` _output_get 0))
      (:`then_1`
        (`WidgetBlueprintLibrary.SetInputMode_GameAndUIEx` self null "DoNotLock" false)))))

(event `Server_PlacePiece`
  (params (Row :type Integer) (Col :type Integer))
  (bind _gamestate (`self.GetPenguinsGameState`))
  (bind _playerstate (`self.GetPenguinsPlayerState`))
  (bind _returnvalue (`PenguinsGameState.PlaceAt` _gamestate (`PenguinsPlayerState.Side` _playerstate) Row Col))
  (`KismetSystemLibrary.PrintText` (`|FormatText` "Placing piece success = {0}" _returnvalue)))

(fn `GetPenguinsGameState`
  (returns (GameState :type "/Game/Blueprints/Penguins/BP_Penguins_GameState Object Reference"))
  (bind _asbp_penguins_game_state (cast `/Game/Blueprints/Penguins/BP_Penguins_GameState` (`GameplayStatics.GetGameState`))
    (:`then`
      (return _asbp_penguins_game_state))
    (:`CastFailed`
      (`KismetSystemLibrary.PrintString` "Failed to cast Game State"))))

(fn `GetPenguinsPlayerState`
  (returns (PlayerState :type "/Game/Blueprints/Penguins/BP_Penguins_PlayerState Object Reference"))
  (bind _asbp_penguins_player_state (cast `/Game/Blueprints/Penguins/BP_Penguins_PlayerState` (`self.PlayerState`))
    (:`then`
      (return _asbp_penguins_player_state))
    (:`CastFailed`
      (`KismetSystemLibrary.PrintString` "Failed to get player state" true true (struct :`R` 1.0 :`B` 0.017792 :`A` 1.0) 10.0))))

(fn `PreLoadSide`
  (bind _playerstate (`self.GetPenguinsPlayerState`))
  (if (`KismetSystemLibrary.IsValid` _playerstate)
    (bind _side (`PenguinsPlayerState.Side` _playerstate))
    (if (`|EnumInequality` _side "Unassigned")
      (`self.UpdateSide` _side))))

(fn `UpdateSide`
  (params (Side :type "EPenguinsSide Enum" :default "Yellow"))
  (bind _hud (`self.HUD`))
  (if (`KismetSystemLibrary.IsValid` _hud)
    (`/Game/Widgets/Penguins/WB_Penguins.UpdateSide` _hud Side)
    (else
      (`KismetSystemLibrary.PrintString` "HUD is invalid"))))

(fn `UserConstructionScript`)