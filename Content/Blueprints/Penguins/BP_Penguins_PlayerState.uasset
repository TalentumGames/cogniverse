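; Player state Blueprint for the Penguins game that passes a player's assigned side to that player's controller.
; On BeginPlay it binds a handler to the side-assigned event.
; When the event fires, the handler casts the owner to the Penguins player controller and calls UpdateSide with the current side, only if that controller is local.
; Debug strings report the handling and the failed checks.
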(event `self.ReceiveBeginPlay`
  (add `self.OnSideAssigned` (delegate `Client_OnSideAssigned`)))

(event `Client_OnSideAssigned`
  (`KismetSystemLibrary.PrintString` "Handling side")
  (`self.HandleSideAssigned`))

(fn `HandleSideAssigned`
  (bind _asbp_penguins_player_controller (cast `/Game/Blueprints/Penguins/BP_Penguins_PlayerController` (`self.GetOwner` self))
    (:`then`
      (if (`Controller.IsLocalPlayerController` _asbp_penguins_player_controller)
        (`/Game/Blueprints/Penguins/BP_Penguins_PlayerController.UpdateSide` _asbp_penguins_player_controller (`self.Side`))
        (else
          (`KismetSystemLibrary.PrintString` "Not a local PC"))))
    (:`CastFailed`
      (`KismetSystemLibrary.PrintString` "Owner is not PC"))))

(fn `UserConstructionScript`)