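; Clickable board slot for the Penguins game, representing one row and column where a player can place a piece.
; Hovering prints a debug name and, if the game state allows placement there, tints the sprite yellow or red for the player's side.
; Leaving resets the tint to white.
; Clicking rechecks validity, then asks the player controller to place the piece on the server.
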(event `self.SpriteComponent.OnBeginCursorOver`
  (params (TouchedComponent :type "PrimitiveComponent Object Reference"))
  (`|ExecutionSequence`
    (:`then_0`
      (`KismetSystemLibrary.PrintString` (`self.GetDebugName` self) true false (struct :`G` 0.66 :`B` 1.0 :`A` 1.0) 2.0 "DebugPiece"))
    (:`then_1`
      (bind _isvalid (`self.IsValidForPlacement`))
      (if _isvalid
        (`self.Highlight`)))))

(event `self.SpriteComponent.OnEndCursorOver`
  (params (TouchedComponent :type "PrimitiveComponent Object Reference"))
  (`self.Unhighlight`))

(event `self.SpriteComponent.OnClicked`
  (params (TouchedComponent :type "PrimitiveComponent Object Reference") (ButtonPressed :type "Key Structure"))
  (`self.AttemptToPlace`))

(fn `AttemptToPlace`
  (bind _isvalid (`self.IsValidForPlacement`))
  (if _isvalid
    (bind _asbp_penguins_player_controller (cast `/Game/Blueprints/Penguins/BP_Penguins_PlayerController` (`GameplayStatics.GetPlayerController` 0)))
    (`/Game/Blueprints/Penguins/BP_Penguins_PlayerController.Server_PlacePiece` _asbp_penguins_player_controller (`self.GetRow`) (`self.GetColumn`))))

(fn `Highlight`
  (switch `EPenguinsSide` (`self.GetMySide`)
    (:`Yellow`
      (`PaperSpriteComponent.SetSpriteColor` (`self.SpriteComponent`) (`self.Yellow`)))
    (:`Red`
      (`PaperSpriteComponent.SetSpriteColor` (`self.SpriteComponent`) (`self.Red`)))))

(fn `IsValidForPlacement`
  (returns (IsValid :type Boolean))
  (bind _asbp_penguins_game_state (cast `/Game/Blueprints/Penguins/BP_Penguins_GameState` (`GameplayStatics.GetGameState`)))
  (return (`PenguinsGameState.CanPlaceAt` _asbp_penguins_game_state (`self.GetMySide`) (`self.GetRow`) (`self.GetColumn`))))

(fn `Unhighlight`
  (`PaperSpriteComponent.SetSpriteColor` (`self.SpriteComponent`) (make `LinearColor` 1.0 1.0 1.0 1.0)))

(fn `UserConstructionScript`)