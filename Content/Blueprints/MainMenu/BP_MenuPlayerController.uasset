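; Main menu player controller that puts up the menu interface and tracks whether the user has logged in.
; On BeginPlay it creates the user HUD and main menu widgets, then sets UI-only input focused on the menu.
; A login callback bound to the HUD sets the LoggedIn flag and prints a confirmation, leaving the received ProductId unused.
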(event `OnLogin`
  (params (ProductId :type String))
  (set `self.LoggedIn` true)
  (`KismetSystemLibrary.PrintString` "Successfully logged in"))

(event `self.ReceiveBeginPlay`
  (`|ExecutionSequence`
    (:`then_0`
      (bind _returnvalue (`|CreateWidget` "/Game/Widgets/MainMenu/WB_UserHUD.WB_UserHUD_C" self))
      (add `/Game/Widgets/MainMenu/WB_UserHUD.LoggedIn` _returnvalue (delegate `OnLogin`))
      (`UserWidget.AddToViewport` _returnvalue 0))
    (:`then_1`
      (bind _returnvalue_2 (`|CreateWidget` "/Game/Widgets/MainMenu/WB_MainMenu.WB_MainMenu_C" self))
      (`UserWidget.AddToViewport` _returnvalue_2 0)
      (`WidgetBlueprintLibrary.SetInputMode_UIOnlyEx` self _returnvalue_2))))

(fn `UserConstructionScript`)