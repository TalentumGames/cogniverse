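; Lobby player controller that shows the lobby UI to the local player and refreshes its list of player names.
; On BeginPlay, only for the local controller, it creates the WB_Lobby widget, adds it to the viewport and switches input to UI-only.
; The PlayersChanged event tells the stored widget, when valid, to update player names, and runs once right after the widget is created.
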(event `self.ReceiveBeginPlay`
  (if (`self.IsLocalPlayerController`)
    (bind _returnvalue (`|CreateWidget` "/Game/Widgets/Lobby/WB_Lobby.WB_Lobby_C" self))
    (`UserWidget.AddToViewport` _returnvalue 0)
    (`WidgetBlueprintLibrary.SetInputMode_UIOnlyEx` self _returnvalue)
    (set `self.LobbyWidget` _returnvalue)
    (`self.PlayersChanged`)))

(event `PlayersChanged`
  (bind _lobbywidget (`self.LobbyWidget`))
  (if (`KismetSystemLibrary.IsValid` _lobbywidget)
    (`/Game/Widgets/Lobby/WB_Lobby.Update Player Names` _lobbywidget)))

(fn `UserConstructionScript`)