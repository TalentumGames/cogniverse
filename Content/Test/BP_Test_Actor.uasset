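; Test actor for checking input and overlap events on an actor and its Sprite component.
; Sprite component click and cursor-over events print debug strings to the screen.
; Actor-level handlers for overlap, cursor-over and click also print strings, but their delegate bindings are unconnected and never run.
; BeginPlay, Tick and the construction script are empty.
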(event `OnActorBeginOverlap_Event` :!signature `self.OnActorBeginOverlap`
  (params (OverlappedActor :type "Actor Object Reference") (OtherActor :type "Actor Object Reference"))
  (`KismetSystemLibrary.PrintString` "Overlap"))

(event `OnBeginCursorOver_Event` :!signature `self.OnBeginCursorOver`
  (params (TouchedActor :type "Actor Object Reference"))
  (`KismetSystemLibrary.PrintString` "Cursor over"))

(event `OnClicked_Event` :!signature `self.OnClicked`
  (params (TouchedActor :type "Actor Object Reference") (ButtonPressed :type "Key Structure" :default "None"))
  (`KismetSystemLibrary.PrintString` "On click"))

(event `self.Sprite.OnClicked`
  (params (TouchedComponent :type "PrimitiveComponent Object Reference") (ButtonPressed :type "Key Structure"))
  (`KismetSystemLibrary.PrintString` "clicked"))

(event `self.Sprite.OnBeginCursorOver`
  (params (TouchedComponent :type "PrimitiveComponent Object Reference"))
  (`KismetSystemLibrary.PrintString` "cursor"))

(fn `UserConstructionScript`)